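; Enemy AI pawn that detects the player, takes damage and explodes on contact.
; PawnSensing sets the "HasSeenPlayer?" blackboard key on its AI controller when it sees a BP_Player.
; Incoming damage lowers HealthEnemy; at zero or below it plays a death sound and explosion, then destroys itself.
; Any capsule overlap also destroys it immediately with explosion effects, without checking what it touched or applying damage.
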(event `self.PawnSensing.OnSeePawn`
  (params (Pawn :type "Pawn Object Reference"))
  (cast `/Game/Game_asset/Playercharacter/BP_Player` Pawn)
  (`BlackboardComponent.SetValueAsBool` (`AIBlueprintHelperLibrary.GetBlackboard` (`AIBlueprintHelperLibrary.GetAIController` self)) "HasSeenPlayer?" true))

(event `self.ReceiveAnyDamage`
  (params (Damage :type "Float (single-precision)") (DamageType :type "DamageType Object Reference") (InstigatedBy :type "Controller Object Reference") (DamageCauser :type "Actor Object Reference"))
  (bind _returnvalue (`self.K2_GetActorLocation`))
  (bind _output_get (set `self.HealthEnemy` (- (`self.HealthEnemy`) Damage)))
  (if (<= _output_get 0.0)
    (`GameplayStatics.PlaySoundAtLocation` "/Game/SoundEffects/enemy_deathAAA.enemy_deathAAA" _returnvalue (struct) 1.0 1.0 0.0 null null null null)
    (`GameplayStatics.SpawnEmitterAtLocation` "/Game/Game_asset/Importedasset/MilitaryWeapSilver/FX/P_RocketLauncher_Explosion_01.P_RocketLauncher_Explosion_01" _returnvalue (struct) (1.0 1.0 1.0) true "AutoRelease")
    (`self.K2_DestroyActor`)))

(event `self.CapsuleComponent.OnComponentBeginOverlap`
  (params (OverlappedComponent :type "PrimitiveComponent Object Reference") (OtherActor :type "Actor Object Reference") (OtherComp :type "PrimitiveComponent Object Reference") (OtherBodyIndex :type Integer) (bFromSweep :type Boolean) (SweepResult :type "HitResult Structure (by ref)"))
  (bind _returnvalue (`self.K2_GetActorLocation`))
  (`GameplayStatics.SpawnEmitterAtLocation` "/Game/StarterContent/Particles/P_Explosion.P_Explosion" _returnvalue (struct) (1.0 1.0 1.0) true "AutoRelease")
  (`GameplayStatics.PlaySoundAtLocation` "/Game/SoundEffects/enemy_deathAAA_Cue.enemy_deathAAA_Cue" _returnvalue (struct) 1.0 1.0 0.0 null null null null)
  (`self.K2_DestroyActor`))

(fn `UserConstructionScript`)