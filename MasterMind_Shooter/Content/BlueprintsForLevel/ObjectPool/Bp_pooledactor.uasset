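; Bp_pooledactor is an object-pool actor that starts disabled and tracks whether it is in use; comments mention bullets.
; SetInUse stores the InUse flag and toggles actor collision to match, and ReturnToPool calls it with false.
; Logic for toggling tick and starting a TimeToLive timer that fires ReturnToPool exists but is disconnected, so nothing here returns the actor automatically.
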(event `self.ReceiveBeginPlay`
  ; all the actors begin in a disabled position
  (`self.SetInUse` false))

(event `SetInUse`
  (params (InUse :type Boolean))
  (set `self.InUse` InUse)
  (`self.SetActorEnableCollision` InUse))

(event `ReturnToPool`
  ; Every certain amount of time the bullets will be rreturned to the pool once the time to live has ended
  (`self.SetInUse` false))

(fn `UserConstructionScript`)