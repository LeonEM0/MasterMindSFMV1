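; Turret Blueprint that tracks BP_Player and fires bullets from two spawn points.
; PawnSensing sightings turn the actor's yaw toward the player with RInterpTo and tilt the Tower within a clamped pitch.
; Each sighting also feeds a chain of retriggerable delays that spawns Bp_bullet at each point in turn and destroys it shortly afterward.
; A Sphere overlap by the player snaps the actor to face them.
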(event `self.PawnSensing.OnSeePawn`
  (params (Pawn :type "Pawn Object Reference"))
  (bind _asbp_player (cast `/Game/Game_asset/Playercharacter/BP_Player` Pawn))
  (`|ExecutionSequence`
    (:`then_0`
      (bind (_returnvalue_roll _returnvalue_pitch _returnvalue_yaw) (`KismetMathLibrary.BreakRotator` (`KismetMathLibrary.RInterpTo` (`self.K2_GetActorRotation`) (`KismetMathLibrary.FindLookAtRotation` (`self.K2_GetActorLocation`) (`self.K2_GetActorLocation` _asbp_player)) (`GameplayStatics.GetWorldDeltaSeconds`) (* 20.0 5.0))))
      (`SceneComponent.K2_SetWorldRotation` (`self.Tower`) (`KismetMathLibrary.MakeRotator` 0.0 (`KismetMathLibrary.FClamp` _returnvalue_pitch -20.0 20.0) _returnvalue_yaw) false false)
      (`self.K2_SetActorRotation` (`KismetMathLibrary.MakeRotator` 0.0 0.0 _returnvalue_yaw)))
    (:`then_1`
      (`KismetSystemLibrary.RetriggerableDelay` 0.2)
      (bind _returnvalue (`|SpawnActorFromClass` "/Game/BlueprintsForLevel/Bullets/Bp_bullet.Bp_bullet_C" (`SceneComponent.K2_GetComponentToWorld` (`self.BulletSpawnPoint1`)) "Undefined" "MultiplyWithRoot" null null))
      (`KismetSystemLibrary.RetriggerableDelay` 0.16)
      (`self.K2_DestroyActor` _returnvalue)
      (bind _returnvalue_2 (`|SpawnActorFromClass` "/Game/BlueprintsForLevel/Bullets/Bp_bullet.Bp_bullet_C" (`SceneComponent.K2_GetComponentToWorld` (`self.BulletSpawnPoint2`)) "Undefined" "MultiplyWithRoot" null null))
      (`KismetSystemLibrary.RetriggerableDelay` 0.16)
      (`self.K2_DestroyActor` _returnvalue_2))))

(event `self.Sphere.OnComponentBeginOverlap`
  (params (OverlappedComponent :type "PrimitiveComponent Object Reference") (OtherActor :type "Actor Object Reference") (OtherComp :type "PrimitiveComponent Object Reference") (OtherBodyIndex :type Integer) (bFromSweep :type Boolean) (SweepResult :type "HitResult Structure (by ref)"))
  (bind _asbp_player (cast `/Game/Game_asset/Playercharacter/BP_Player` OtherActor))
  (bind (_returnvalue_roll _returnvalue_pitch _returnvalue_yaw) (`KismetMathLibrary.BreakRotator` (`KismetMathLibrary.FindLookAtRotation` (`self.K2_GetActorLocation`) (`self.K2_GetActorLocation` _asbp_player))))
  (`self.K2_SetActorRotation` (`KismetMathLibrary.MakeRotator` 0.0 _returnvalue_pitch _returnvalue_yaw)))

(fn `UserConstructionScript`)