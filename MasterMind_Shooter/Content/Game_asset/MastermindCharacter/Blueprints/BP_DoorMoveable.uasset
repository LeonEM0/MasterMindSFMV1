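; BP_DoorMoveable is a sliding door that toggles between two positions when its custom event is called.
; Each call eases the Object component 225 units along its relative X axis over one second, alternating direction via BIsOpen.
; BMoveCompleted blocks new toggles until the move finishes, then Open or Close is printed.
; BIsOpen reads inverted: the branch that prints Open sets it to false.
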(event `CustomEvent`
  (bind _object (`self.Object`))
  (bind _relativelocation (`SceneComponent.RelativeLocation` (`self.Object`)))
  (if (`self.b_MoveCompleted`)
    (if (`self.b_isOpen`)
      (bind _output_get (set `self.v_TargetLocation` _relativelocation))
      (set `self.b_isOpen` false)
      (set `self.b_MoveCompleted` false)
      (`KismetSystemLibrary.MoveComponentTo` _object (+ _output_get (225.0 0.0 0.0)) (struct) true true 1.0)
      (set `self.b_MoveCompleted` true)
      (`KismetSystemLibrary.PrintText` "Open")
      (else
        (bind _output_get_2 (set `self.v_TargetLocation` _relativelocation))
        (set `self.b_isOpen` true)
        (set `self.b_MoveCompleted` false)
        (`KismetSystemLibrary.MoveComponentTo` _object (- _output_get_2 (225.0 0.0 0.0)) (struct) true true 1.0)
        (set `self.b_MoveCompleted` true)
        (`KismetSystemLibrary.PrintText` "Close")))))

(fn `UserConstructionScript`
  (`parent.UserConstructionScript`))