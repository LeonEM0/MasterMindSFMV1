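; BP_SpeedPickup is a pickup that raises the walk speed of the pawn that collects it.
; Its Pickup event finds the pawn's CharacterMovementComponent and adds SpeedIncreaseAmount to MaxWalkSpeed, printing debug messages around a five-second delay.
; The post-delay step re-reads the current speed, then adds and subtracts the same amount, so the boost is never actually removed.
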(event `self.Pickup`
  (params (PlayerPawn :type "Pawn Object Reference"))
  (bind _returnvalue (`self.GetComponentByClass` PlayerPawn "/Script/Engine.CharacterMovementComponent"))
  (bind _speedincreaseamount (`self.SpeedIncreaseAmount`))
  (bind _returnvalue_2 (+ (`CharacterMovementComponent.MaxWalkSpeed` _returnvalue) _speedincreaseamount))
  (`/Engine/EditorBlueprintResources/StandardMacros.IsValid` _returnvalue
    (:`Is Valid`
      (set `CharacterMovementComponent.MaxWalkSpeed` _returnvalue_2 _returnvalue)
      (`KismetSystemLibrary.PrintString` "Speed Increase Begin")
      (`KismetSystemLibrary.Delay` 5.0)
      (set `CharacterMovementComponent.MaxWalkSpeed` (- _returnvalue_2 _speedincreaseamount) _returnvalue)
      (`KismetSystemLibrary.PrintString` "Speed Increase End"))))

(fn `UserConstructionScript`
  (`parent.UserConstructionScript`))